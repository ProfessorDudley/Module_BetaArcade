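; Side trampoline environment Blueprint that launches HP_CH_Player characters and plays a jump cue when their capsule overlaps its Box.
; Launch velocity adds large fixed offsets to the Direction component's forward vector, randomizing X, negating Y and lifting Z, then scales by LaunchStrength.
; The offsets outweigh the unit vector, so rotating Direction barely changes the launch, which overrides existing XY and Z velocity.
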(event `self.Box.OnComponentBeginOverlap`
  (params (OverlappedComponent :type "PrimitiveComponent Object Reference") (OtherActor :type "Actor Object Reference") (OtherComp :type "PrimitiveComponent Object Reference") (OtherBodyIndex :type Integer) (bFromSweep :type Boolean) (SweepResult :type "HitResult Structure (by ref)"))
  (bind _x (.x (`SceneComponent.GetForwardVector` (`self.Direction`))))
  ;[1 1 1] Launch
  (if (== (`GameplayStatics.GetObjectClass` OtherComp) "/Script/Engine.CapsuleComponent")
    (bind _ashp_ch_player (cast `HP_CH_Player` OtherActor))
    (`Character.LaunchCharacter` _ashp_ch_player (* (`KismetMathLibrary.MakeVector` (`KismetMathLibrary.RandomFloatInRange` (- _x 15.0) (+ _x 15.0)) (* (+ (.y (`SceneComponent.GetForwardVector` (`self.Direction`))) 15.0) -1.0) (+ (.z (`SceneComponent.GetForwardVector` (`self.Direction`))) 15.0)) (`self.LaunchStrength`)) true true)
    (`GameplayStatics.PlaySoundAtLocation` "/Game/HotPotato/Audio/SoundFX/Jump_-_Trampoline_Cue.Jump_-_Trampoline_Cue" (`.Location` (`GameplayStatics.BreakHitResult` SweepResult)))))

(fn `UserConstructionScript`)