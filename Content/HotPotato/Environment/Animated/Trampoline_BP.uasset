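; Trampoline actor for Hot Potato that gives players a different jump strength while they stand on it.
; When a player character's capsule begins overlapping the Box, it sets the CharacterMovement JumpZVelocity to BounceJump, and restores BaseJump when the capsule leaves.
; The capsule class check ignores other components, and debug prints mark entry and exit.
; It only alters jump velocity and applies no launch itself.
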(event `self.Box.OnComponentBeginOverlap`
  (params (OverlappedComponent :type "PrimitiveComponent Object Reference") (OtherActor :type "Actor Object Reference") (OtherComp :type "PrimitiveComponent Object Reference") (OtherBodyIndex :type Integer) (bFromSweep :type Boolean) (SweepResult :type "HitResult Structure (by ref)"))
  ;[1 1 1] Check if the player is fully on the trampoline.
  (if (== (`GameplayStatics.GetObjectClass` OtherComp) "/Script/Engine.CapsuleComponent")
    (bind _ashp_ch_player (cast `HP_CH_Player` OtherActor)) ; Check to see if the actor is a player
    ;[1 1 1] Set the Jump ZVelocity
    (set `CharacterMovementComponent.JumpZVelocity` (`self.BounceJump`) (`Character.CharacterMovement` _ashp_ch_player))
    (`KismetSystemLibrary.PrintString` "in")))

(event `self.Box.OnComponentEndOverlap`
  (params (OverlappedComponent :type "PrimitiveComponent Object Reference") (OtherActor :type "Actor Object Reference") (OtherComp :type "PrimitiveComponent Object Reference") (OtherBodyIndex :type Integer))
  ;[1 1 1] Check if the player is fully off the trampoline.
  (if (== (`GameplayStatics.GetObjectClass` OtherComp) "/Script/Engine.CapsuleComponent")
    (bind _ashp_ch_player (cast `HP_CH_Player` OtherActor)) ; Check to see if the actor is a player
    ;[1 1 1] Reset the Jump ZVelocity
    (set `CharacterMovementComponent.JumpZVelocity` (`self.BaseJump`) (`Character.CharacterMovement` _ashp_ch_player))
    (`KismetSystemLibrary.PrintString` "out")))

(fn `UserConstructionScript`)