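; Barbara character Blueprint for Hot Potato, handling jump feedback, walking dust and a player indicator ring.
; Jump input plays a sound and pauses mesh animation until landing triggers a brief dust burst.
; Tick toggles walk dust through paired DoOnce gates and line-traces downward to keep the ring on the floor.
; BeginPlay loops over HP_CH_Player actors, overwriting its own ring material and stencil value by index, so the last match wins.
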(event `self.ReceiveTick`
  (params (DeltaSeconds :type "Float (single-precision)"))
  (bind _walkdust (`self.WalkDust`))
  (bind (_velocity_x _velocity_y) (`KismetMathLibrary.BreakVector` (`MovementComponent.Velocity` (`self.CharacterMovement`))))
  ;[1 1 1] WalkingDust
  (`|ExecutionSequence`
    (:`then_0`
      (if (`self.IsJumping`)
        _
        (elif (or (!= _velocity_x 0.0) (!= _velocity_y 0.0))
          (`/Engine/EditorBlueprintResources/StandardMacros.DoOnce` false :!label _label
            (:`Completed`
              (`ActorComponent.Activate` _walkdust false)
              (goto _label_2 :!via `Reset`)))
          (else
            _)))
      (`/Engine/EditorBlueprintResources/StandardMacros.DoOnce` false :!label _label_2
        (:`Completed`
          (`ActorComponent.Deactivate` _walkdust)
          (goto _label :!via `Reset`))))
    (:`then_1`
      (`self.UpdateRing`))))

(event `InputAction|Jump`
  (params (Key :type "Key Structure"))
  ;[1 1 1] Jumping
  (:`Pressed`
    (if (not (`NavMovementComponent.IsFalling` (`self.CharacterMovement`)))
      (`self.Jump`)
      (set `self.IsJumping` true)
      (set `SkeletalMeshComponent.bPauseAnims` true (`self.Mesh`))
      (`GameplayStatics.PlaySoundAtLocation` "/Game/HotPotato/Audio/SoundFX/JumpingCue.JumpingCue" (`SceneComponent.K2_GetComponentLocation` (`self.Mesh`))))))

(event `self.OnLanded`
  (params (Hit :type "HitResult Structure (by ref)"))
  (bind _landingdust (`self.LandingDust`))
  ;[1 1 1] Jumping
  (set `self.IsJumping` false)
  (set `SkeletalMeshComponent.bPauseAnims` false (`self.Mesh`))
  (`ActorComponent.Activate` _landingdust false)
  (`KismetSystemLibrary.Delay` 0.2)
  (`ActorComponent.Deactivate` _landingdust))

(event `self.ReceiveBeginPlay`
  (bind _mesh (`self.Mesh`))
  (bind _playerring (`self.PlayerRing`))
  ;[1 1 1] Setting player ring colour
  (bind _outactors (`GameplayStatics.GetAllActorsOfClass` "/Script/HotPotato.HP_CH_Player"))
  (for (_ _array_index) _outactors
    (switch `int` _array_index
      (:`0`
        (`PrimitiveComponent.SetMaterial` _playerring 0 "/Game/HotPotato/Art/Particles/PlayerRing/Player1Ring_Mat_Inst.Player1Ring_Mat_Inst")
        (`PrimitiveComponent.SetCustomDepthStencilValue` _mesh 1))
      (:`1`
        (`PrimitiveComponent.SetMaterial` _playerring 0 "/Game/HotPotato/Art/Particles/PlayerRing/Player2Ring_Mat_Inst.Player2Ring_Mat_Inst")
        (`PrimitiveComponent.SetCustomDepthStencilValue` _mesh 2))
      (:`2`
        (`PrimitiveComponent.SetMaterial` _playerring 0 "/Game/HotPotato/Art/Particles/PlayerRing/Player3Ring_Mat_Inst.Player3Ring_Mat_Inst")
        (`PrimitiveComponent.SetCustomDepthStencilValue` _mesh 3))
      (:`3`
        (`PrimitiveComponent.SetMaterial` _playerring 0 "/Game/HotPotato/Art/Particles/PlayerRing/Player4Ring_Mat_Inst.Player4Ring_Mat_Inst")
        (`PrimitiveComponent.SetCustomDepthStencilValue` _mesh 4)))))

(event `UpdateRing`
  (bind _playerring (`self.PlayerRing`))
  (bind (_returnvalue_x _returnvalue_y) (`KismetMathLibrary.BreakVector` (`SceneComponent.K2_GetComponentLocation` _playerring)))
  (bind _returnvalue (`SceneComponent.K2_GetComponentLocation` (`self.Mesh`)))
  ;[1 1 1] Keep player ring on floor
  (bind _outhit (`KismetSystemLibrary.LineTraceSingle` _returnvalue (`KismetMathLibrary.MakeVector` (.x _returnvalue) (.y _returnvalue) (- (.z _returnvalue) 8000.0)) "TraceTypeQuery1"))
  (`SceneComponent.K2_SetWorldLocation` _playerring (`KismetMathLibrary.MakeVector` _returnvalue_x _returnvalue_y (+ (.z (`.Location` (`GameplayStatics.BreakHitResult` _outhit))) 1.0)) false false))

(fn `UserConstructionScript`)