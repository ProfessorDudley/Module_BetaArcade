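; BP_Mask_Fish is the fish mask in the HotPotato game, reacting when it is equipped or dequipped.
; On equip it copies the owner mesh's custom depth stencil value onto its own mesh and plays a zip sound at the mask's location.
; On dequip it resets the mask's stencil value to zero.
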(event `self.AfterTheMaskIsEquipped`
  ;[1 1 1] Set Stencil Depth = Player
  (`PrimitiveComponent.SetCustomDepthStencilValue` (`self.Mesh`) (`PrimitiveComponent.CustomDepthStencilValue` (`Character.Mesh` (`self.owner_`))))
  (`GameplayStatics.PlaySoundAtLocation` "/Game/HotPotato/Audio/SoundFX/Mask_-_Zip_1_Cue.Mask_-_Zip_1_Cue" (`SceneComponent.K2_GetComponentLocation` (`self.Mesh`))))

(event `self.AfterTheMaskIsDequipped`
  ;[1 1 1] Remove Stencil Depth
  (`PrimitiveComponent.SetCustomDepthStencilValue` (`self.Mesh`) 0))

(fn `UserConstructionScript`)